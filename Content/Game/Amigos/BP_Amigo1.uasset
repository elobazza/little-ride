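; Collectible friend (amigo) that the player's BP_BaseCar picks up by dealing damage to it, raising the car's collected count.
; After a delay, a count of four shows the victory HUD, pauses the game and deletes the Checkpoint save.
; Otherwise it destroys itself and calls SalvarCheckpoint, which uses DoOnce to write the car's stats, timer, count and transform to the Checkpoint slot.
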(event `self.ReceiveAnyDamage`
  (params (Damage :type "Float (single-precision)") (DamageType :type "DamageType Object Reference") (InstigatedBy :type "Controller Object Reference") (DamageCauser :type "Actor Object Reference"))
  (bind _asbp_base_car (cast `/Game/DriveableCar_basic/Blueprints/Vehicles/BP_BaseCar` DamageCauser))
  (bind _output_get (set `/Game/DriveableCar_basic/Blueprints/Vehicles/BP_BaseCar.qtdAmigosRecolhidos` (+ (`/Game/DriveableCar_basic/Blueprints/Vehicles/BP_BaseCar.qtdAmigosRecolhidos` _asbp_base_car) 1) _asbp_base_car))
  (`KismetSystemLibrary.Delay` 2.0)
  (if (== _output_get 4)
    (`KismetSystemLibrary.Delay` 1.0)
    (bind _returnvalue (`|CreateWidget` "/Game/Game/HUDs/HUD_Vitoria.HUD_Vitoria_C"))
    (`UserWidget.AddToViewport` _returnvalue 0)
    (`GameplayStatics.SetGamePaused` true)
    (set `PlayerController.bShowMouseCursor` true (`GameplayStatics.GetPlayerController` 0))
    (`GameplayStatics.DeleteGameInSlot` (`self.Checkpoint`))
    (else
      (`self.K2_DestroyActor`)
      (`self.SalvarCheckpoint`))))

(event `SalvarCheckpoint`
  (bind _checkpoint (`self.Checkpoint`))
  (`/Engine/EditorBlueprintResources/StandardMacros.DoOnce` false
    (:`Completed`
      (bind _returnvalue (`GameplayStatics.CreateSaveGameObject` "/Game/Game/Checkpoint/BP_SaveGame.BP_SaveGame_C"))
      (bind _output_get (set `self.SubClass` _returnvalue))
      (bind _asbp_save_game (cast `/Game/Game/Checkpoint/BP_SaveGame` _output_get))
      (bind _asbp_base_car (cast `/Game/DriveableCar_basic/Blueprints/Vehicles/BP_BaseCar` (`GameplayStatics.GetPlayerPawn` 0)))
      (set `/Game/Game/Checkpoint/BP_SaveGame.VidaSave` (`/Game/DriveableCar_basic/Blueprints/Vehicles/BP_BaseCar.Vida` _asbp_base_car) _asbp_save_game)
      (set `/Game/Game/Checkpoint/BP_SaveGame.GasolinaSave` (`/Game/DriveableCar_basic/Blueprints/Vehicles/BP_BaseCar.Gasolina` _asbp_base_car) _asbp_save_game)
      (set `/Game/Game/Checkpoint/BP_SaveGame.qtdVidaUsadaSave` (`/Game/DriveableCar_basic/Blueprints/Vehicles/BP_BaseCar.qtdVidaUsada` _asbp_base_car) _asbp_save_game)
      (set `/Game/Game/Checkpoint/BP_SaveGame.qtdGasolinaUsadaSave` (`/Game/DriveableCar_basic/Blueprints/Vehicles/BP_BaseCar.qtdGasolinaUsada` _asbp_base_car) _asbp_save_game)
      (set `/Game/Game/Checkpoint/BP_SaveGame.qtdAmigosRecolhidosSave` (`/Game/DriveableCar_basic/Blueprints/Vehicles/BP_BaseCar.qtdAmigosRecolhidos` _asbp_base_car) _asbp_save_game)
      (set `/Game/Game/Checkpoint/BP_SaveGame.MinutosSave` (`/Game/DriveableCar_basic/Blueprints/Vehicles/BP_BaseCar.Minutos` _asbp_base_car) _asbp_save_game)
      (set `/Game/Game/Checkpoint/BP_SaveGame.SegundosSave` (`/Game/DriveableCar_basic/Blueprints/Vehicles/BP_BaseCar.Segundos` _asbp_base_car) _asbp_save_game)
      (bind (_returnvalue_location _returnvalue_rotation _returnvalue_scale) (`KismetMathLibrary.BreakTransform` (`self.GetTransform` _asbp_base_car)))
      (set `/Game/Game/Checkpoint/BP_SaveGame.PlayerLocationSave` (`KismetMathLibrary.MakeTransform` _returnvalue_location _returnvalue_rotation _returnvalue_scale) _asbp_save_game)
      (bind _returnvalue_2 (`GameplayStatics.DoesSaveGameExist` (`self.Checkpoint`)))
      (if _returnvalue_2
        (`GameplayStatics.DeleteGameInSlot` _checkpoint)
        (`GameplayStatics.SaveGameToSlot` (`self.SubClass`) _checkpoint)
        (else
          (`GameplayStatics.SaveGameToSlot` (`self.SubClass`) (`self.Checkpoint`))))
      (`KismetSystemLibrary.PrintString` "Realizado Checkpoint!"))))

(fn `UserConstructionScript`)