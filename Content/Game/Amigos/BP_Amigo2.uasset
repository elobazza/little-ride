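; BP_Amigo2 is a collectible friend ("amigo") actor that a BP_BaseCar picks up by damaging it.
; AnyDamage casts the damage causer to the car, increments its QtdAmigosRecolhidos count, then destroys the amigo after a short delay.
; When the count equals four, a further Delay, placed after DestroyActor, leads to showing HUD_Vitoria, pausing the game and showing the mouse cursor.
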(event `self.ReceiveAnyDamage`
  (params (Damage :type "Float (single-precision)") (DamageType :type "DamageType Object Reference") (InstigatedBy :type "Controller Object Reference") (DamageCauser :type "Actor Object Reference"))
  (bind _asbp_base_car (cast `/Game/DriveableCar_basic/Blueprints/Vehicles/BP_BaseCar` DamageCauser))
  (bind _output_get (set `/Game/DriveableCar_basic/Blueprints/Vehicles/BP_BaseCar.qtdAmigosRecolhidos` (+ (`/Game/DriveableCar_basic/Blueprints/Vehicles/BP_BaseCar.qtdAmigosRecolhidos` _asbp_base_car) 1) _asbp_base_car))
  (`KismetSystemLibrary.Delay` 2.0)
  (`self.K2_DestroyActor`)
  (if (== _output_get 4)
    (`KismetSystemLibrary.Delay` 1.0)
    (bind _returnvalue (`|CreateWidget` "/Game/Game/HUDs/HUD_Vitoria.HUD_Vitoria_C"))
    (`UserWidget.AddToViewport` _returnvalue 0)
    (`GameplayStatics.SetGamePaused` true)
    (set `PlayerController.bShowMouseCursor` true (`GameplayStatics.GetPlayerController` 0))))

(fn `UserConstructionScript`)